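; BP_Character is a first-person player character with look, walk and hold-to-run controls and a single hand slot for carrying an item.
; Left click line-traces from the camera and sends PlayerInteractedMessage to a hit actor that also overlaps the character and implements the player interaction interface.
; AddtoHand fills the slot with a mesh and string only when the hand is free, and EmptyHand clears it.
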(event EventEmptyHand
  ;[1 1 1] Empty Hand
  (bind _output_get (Variables|Default|SetOnHandMesh 0))
  (Variables|Default|SetHandFull? false)
  (Variables|Default|SetOnHandString "")
  (Components|StaticMesh|SetStaticMesh (Variables|Default|GetOnHand) _output_get))

(event EventAddtoHand
  (params (ToHandMesh :type Static%20Mesh%20Object%20Reference) (ToHandString :type String))
  ;[1 1 1] Add to Hand
  (if (not (Variables|Default|GetHandFull?))
    (Components|StaticMesh|SetStaticMesh (Variables|Default|GetOnHand) ToHandMesh)
    (Variables|Default|SetOnHandString ToHandString)
    (Variables|Default|SetHandFull? true)
    (Variables|Default|SetOnHandMesh ToHandMesh)))

(event Input|ActionEvents|InputActionRun
  (params (Key :type Key%20Structure :default "None"))
  (bind _runspeed (Variables|Default|GetRunSpeed))
  (bind _charactermovement (Variables|Character|GetCharacterMovement))
  ;[1 1 1] Basic Controllers
  ;;[1 1 1] Run
  (:Pressed
    (Variables|/Script/Engine.CharacterMovementComponent|SetMaxWalkSpeed _charactermovement (* (Variables|/Script/Engine.CharacterMovementComponent|GetMaxWalkSpeed (Variables|Character|GetCharacterMovement)) _runspeed)))
  (:Released
    (Variables|/Script/Engine.CharacterMovementComponent|SetMaxWalkSpeed _charactermovement (/ (Variables|/Script/Engine.CharacterMovementComponent|GetMaxWalkSpeed (Variables|Character|GetCharacterMovement)) _runspeed))))

(event Input|ActionEvents|InputActionLeft_click
  (params (Key :type Key%20Structure :default "None"))
  (bind _camera (Variables|Default|GetCamera))
  (bind _returnvalue (Transformation|GetWorldLocation _camera))
  ;[1 1 1 1 97] On Left Click
  (:Pressed
    ;;[1 1 1] Line trace
    (bind _outhit (Collision|LineTraceByChannel _returnvalue (+ _returnvalue (* (Math|Vector|GetForwardVector (Transformation|GetWorldRotation _camera)) 1.5e+03)) "TraceTypeQuery1" false 0 "None"))
    ;;[1 1 1] Check Overlap & Check Interface
    (for _array_element (Collision|GetOverlappingActors 0 :!class /Script/Engine.Actor)
      (if (and (== (.HitActor (Collision|BreakHitResult _outhit)) _array_element) (Utilities|DoesObjectImplementInterface _array_element "/Game/_Main/BP_Player_Interaction_Interface.BP_Player_Interaction_Interface_C"))
        (Class|BPPlayerInteractionInterface|PlayerInteracted(Message) _array_element self)))))

(event Input|AxisEvents|InputAxisMove_Y
  (params (AxisValue :type Float%20%28single-precision%29))
  ;[1 1 1] Basic Controllers
  ;;[1 1 1] Walk
  (Pawn|Input|AddMovementInput (Transformation|GetActorForwardVector) AxisValue false))

(event Input|AxisEvents|InputAxisMove_X
  (params (AxisValue :type Float%20%28single-precision%29))
  ;[1 1 1] Basic Controllers
  ;;[1 1 1] Walk
  (Pawn|Input|AddMovementInput (Transformation|GetActorRightVector) AxisValue false))

(event Input|AxisEvents|InputAxisLook_X
  (params (AxisValue :type Float%20%28single-precision%29))
  ;[1 1 1] Basic Controllers
  ;;[1 1 1] Look
  (Pawn|Input|AddControllerYawInput AxisValue))

(event Input|AxisEvents|InputAxisLook_Y
  (params (AxisValue :type Float%20%28single-precision%29))
  ;[1 1 1] Basic Controllers
  ;;[1 1 1] Look
  (Pawn|Input|AddControllerPitchInput AxisValue))

(fn ConstructionScript)