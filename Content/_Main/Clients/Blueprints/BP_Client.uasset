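; AI customer character that orders a sandwich, queues at a BP_Sandwich and reports a score to the game mode.
; Construction script builds a bread-bookended order from placed BP_Ingredient actors and joins a random sandwich queue.
; It walks over, slowing on approach, with the order in a bubble widget.
; Tick-driven impatience speeds up on arrival, adding red-shift material and smoke until timeout triggers a penalty and exit to despawn.
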(event Custom|NewOrder
  ;[1 1 1] Generate a New Order
  (Variables|Default|SetFillingAmount (+ (Math|Random|RandomInteger 4) 1))
  (bind _randombread (CallFunction|GetRandomBread))
  (Utilities|Array|Add (Variables|Default|GetClientOrder) (Utilities|Array|Get(acopy) (Variables|Default|GetBreadTypes) _randombread))
  (while (> (Variables|Default|GetFillingAmount) 0)
    (bind _randomfilling (CallFunction|GetRandomFilling))
    (Utilities|Array|Add (Variables|Default|GetClientOrder) (Utilities|Array|Get(acopy) (Variables|Default|GetFillingTypes) _randomfilling))
    (Variables|Default|SetFillingAmount (- (Variables|Default|GetFillingAmount) 1)))
  (Utilities|Array|Add (Variables|Default|GetClientOrder) (Utilities|Array|Get(acopy) (Variables|Default|GetBreadTypes) _randombread)))

(event Custom|AttachToSandwich
  ;[1 1 1] Attach To Sandwich
  (bind _outactors (Actor|GetAllActorsOfClass "/Game/_Main/Orders/Blueprints/BP_Sandwich.BP_Sandwich_C"))
  (bind _output_get (Variables|Default|SetSandwich (Utilities|Array|Get(acopy) _outactors (Math|Random|RandomInteger (- (Utilities|Array|Length _outactors) 1)))))
  (Default|AddClienttoQueue _output_get self))

(event Custom|InitializeBreadsFillings
  ;[1 1 1] Get all the breads and fillings
  (bind _outactors (Actor|GetAllActorsOfClass "/Game/_Main/Ingredients/Blueprints/BP_Ingredient.BP_Ingredient_C"))
  (for _array_element _outactors
    (if (Variables|/Game/_Main/Ingredients/Blueprints/BP_Ingredient.BP_Ingredient_C|GetIsBread? _array_element)
      (Utilities|Array|Add (Variables|Default|GetBreadTypes) (Variables|/Game/_Main/Ingredients/Blueprints/BP_Ingredient.BP_Ingredient_C|GetIngredientName _array_element))
      (else
        (Utilities|Array|Add (Variables|Default|GetFillingTypes) (Variables|/Game/_Main/Ingredients/Blueprints/BP_Ingredient.BP_Ingredient_C|GetIngredientName _array_element))))))

(event Custom|UpdateBubble
  ;[1 1 1] Update speech bubble
  (bind _aswb_order_bubble (Utilities|Casting|CastToWB_Order_Bubble (UserInterface|GetUserWidgetObject (Variables|Default|GetWidget))))
  (Variables|/Game/_Main/Clients/WB_Order_Bubble.WB_Order_Bubble_C|SetOrderString _aswb_order_bubble (Utilities|String|JoinStringArray (Variables|Default|GetClientOrder) " ")))

(event Custom|LeaveScene
  (Rendering|ToggleVisibility (Variables|Default|GetWidget) false)
  (bind _outactors (Actor|GetAllActorsOfClass "/Game/_Main/Clients/Blueprints/BP_Despawn_Point.BP_Despawn_Point_C"))
  (AI|AIMoveTo self "0, 0, 0" (.OutItem (Utilities|Array|Random _outactors)) 5.0 false
    (:OnSuccess
      (Actor|DestroyActor))))

(event Custom|PissedOff
  (CallFunction|IncorrectOrder)
  (CallFunction|LeaveScene))

(event Custom|CalculateScore
  ;[1 1 1] Score calculator
  (if (Variables|Default|GetOrderCorrect?)
    (Variables|Default|SetTotalScore (Math|Conversions|ToFloat(Integer) (|((({2999A115-40D1-DAB0-5763-75A35F9085D2}/{5722D6AC-443C-6EEF-FEE8-8C965A96F859})*{97257AB6-45D7-DE45-2671-E3A44C4792DC})+{C3954F25-43AE-5275-B4AE-D495523830D2}))))
    (else
      (Variables|Default|SetTotalScore (- 0.0 (Math|Conversions|ToFloat(Integer) (|({C3954F25-43AE-5275-B4AE-D495523830D2}/2))))))))

(event Custom|Impatience%20Countdown
  ;[1 1 1] Clock in miliseconds
  (if (not (Variables|Default|GetIsPissedOf?))
    (Utilities|FlowControl|Delay (/ (Variables|Default|GetTimePatienceDrop) (Variables|Default|GetImpatienceRate)))
    (Variables|Default|SetSpawnTime (+ (Variables|Default|GetSpawnTime) 1))
    (if (> (Variables|Default|GetSpawnTime) (Variables|Default|GetPatience))
      (Variables|Default|SetIsPissedOf? true)
      (CallFunction|PissedOff)
      (else
        (CallFunction|VisualizeImpatience)))))

(event Custom|DetermineWalkSpeed
  (bind _returnvalue (Transformation|GetActorLocation))
  (bind _sandwich (Variables|Default|GetSandwich))
  (bind _currentclientlocation (Variables|/Game/_Main/Orders/Blueprints/BP_Sandwich.BP_Sandwich_C|GetCurrentClientLocation _sandwich))
  (bind _returnvalue_2 (Transformation|GetActorLocation _currentclientlocation))
  (bind _returnvalue_3 (Math|Vector|Distance(Vector) _returnvalue _returnvalue_2))
  ;[1 1 1] Event that lowers walk speed as it gets close to final location
  (if (< _returnvalue_3 7e+02)
    (Variables|/Script/Engine.CharacterMovementComponent|SetMaxWalkSpeed (Variables|Character|GetCharacterMovement) (|(((pow((x/700),2))*300)+300) _returnvalue_3))))

(event Custom|VisualizeImpatience
  (if (Variables|Default|GetIsShaking?)
    _
    (else
      _))
  ;[1 1 1] Event in charge of changing color and adding particles
  (Rendering|Material|SetVectorParameterValue (Variables|Default|GetMaterial) "AngryColorTransparency" (Math|Conversions|ToLinearColor(Vector) (/ (Variables|Default|GetSpawnTime) (Variables|Default|GetPatience))) :!class /Script/Engine.MaterialInstanceDynamic)
  (if (and (> (/ (Variables|Default|GetSpawnTime) (Variables|Default|GetPatience)) 0.8) (|({96AFAFBC-46C5-D6D1-2F7A-F49A8CD827C9}<2)))
    (Effects|SpawnEmitterAttached "/Game/Fantastic_Village_Pack/effects/PS_FX_smoke.PS_FX_smoke" (Variables|Collision|GetCapsuleComponent) "None" "0, 0,10.000000")
    (Variables|Default|SetSmokey 2)
    (elif (and (> (/ (Variables|Default|GetSpawnTime) (Variables|Default|GetPatience)) 0.4) (|({96AFAFBC-46C5-D6D1-2F7A-F49A8CD827C9}<1)))
      (Effects|SpawnEmitterAttached "/Game/UndeadPack/SkeletonEnemy/Particles/P_Smoke_FX.P_Smoke_FX" (Variables|Collision|GetCapsuleComponent) "None" "0, 0,10.000000")
      (Variables|Default|SetSmokey 1)
      (Variables|Default|SetIsShaking? true))))

(event EventCorrectOrder
  ;[1 1 1] On Sent Order from Sandwich
  (Variables|Default|SetOrderCorrect? true)
  (CallFunction|CalculateScore)
  (Class|BPIncreaseScoreInterface|PushScoreChange(Message) (Game|GetGameMode) (Variables|Default|GetTotalScore)))

(event EventBeginPlay
  ;[1 1 1] At Spawn
  (bind _returnvalue (Rendering|Material|CreateDynamicMaterialInstance (Variables|Character|GetMesh) 0 "/Game/UndeadPack/EnemyGoblin/Materials/M_EnemyGoblin_01.M_EnemyGoblin_01" "None" :!class /Script/Engine.PrimitiveComponent))
  (Variables|Default|SetMaterial _returnvalue)
  (AI|AIMoveTo self "0, 0, 0" (Variables|/Game/_Main/Orders/Blueprints/BP_Sandwich.BP_Sandwich_C|GetCurrentClientLocation (Variables|Default|GetSandwich)) 5.0 false
    (:then
      (CallFunction|UpdateBubble))
    (:OnSuccess
      (Rendering|ToggleVisibility (Variables|Default|GetWidget) false)
      (Variables|Default|SetImpatienceRate (* (Variables|Default|GetImpatienceRate) 1e+01)))))

(event EventTick
  (params (DeltaSeconds :type Float%20%28single-precision%29))
  (CallFunction|DetermineWalkSpeed)
  (CallFunction|ImpatienceCountdown))

(event EventIncorrectOrder
  ;[1 1 1] On Sent Order from Sandwich
  (Variables|Default|SetOrderCorrect? false)
  (CallFunction|CalculateScore)
  (Class|BPIncreaseScoreInterface|PushScoreChange(Message) (Game|GetGameMode) (Variables|Default|GetTotalScore)))

(fn ConstructionScript
  (CallFunction|InitializeBreadsFillings)
  (CallFunction|NewOrder)
  (CallFunction|AttachtoSandwich)
  (Rendering|SetVisibility (Variables|Default|GetWidget) false false))

(fn GetRandomBread
  (return 0))

(fn GetRandomFilling
  (return (Math|Random|RandomInteger (Utilities|Array|Length (Variables|Default|GetFillingTypes)))))

(fn NewFunction0)