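; BP_Sandwich is the plate where the player assembles sandwiches to fill orders from a queue of clients.
; Interacting empties the player's hand, stacking the held mesh as a new component at a height accumulated from bounding boxes and recording its ingredient string.
; SubmitSandwich compares the joined built strings with the front client's order, so sequence matters, then triggers that client's correct or incorrect message.
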(event Custom|AddToSandwich
  (params (PlayerCharacter :type BP%20Character%20Object%20Reference))
  ;[1 1 1] Add To Sandwich
  (if (Variables|/Game/_Main/Player/BP_Character.BP_Character_C|GetHandFull? PlayerCharacter) ; Check Player's hand is full
    (Variables|Default|SetIngredientMesh (Variables|/Game/_Main/Player/BP_Character.BP_Character_C|GetOnHandMesh PlayerCharacter))
    (Utilities|Array|Add (Variables|Default|GetBuiltSandwich) (Variables|/Game/_Main/Player/BP_Character.BP_Character_C|GetOnHandString PlayerCharacter))
    (bind _returnvalue (AddComponent|AddStaticMeshComponent false (Variables|Default|GetNextMeshPosition)))
    (Components|StaticMesh|SetStaticMesh _returnvalue (Variables|Default|GetIngredientMesh))
    (Variables|Default|SetNextMeshPosition (Math|Transform|MakeTransform (Math|Vector|MakeVector 0.0 0.0 (+ (.Z (Class|KismetMathLibrary|BreakVector3f (.Location (Math|Transform|BreakTransform (Variables|Default|GetNextMeshPosition))))) (.Z (Class|KismetMathLibrary|BreakVector3f (.Max (Utilities|Struct|BreakBox (StaticMesh|GetBoundingBox (Variables|Default|GetIngredientMesh))))))))))))

(event Custom|CompareSandwiches
  (bind _clientqueue (Variables|Default|GetClientQueue))
  (bind _output (Utilities|Array|Get(acopy) _clientqueue))
  ;[1 1 1] Compares Sandwiches
  (if (Utilities|Enum|Equal(Enum) (Utilities|String|JoinStringArray (Variables|Default|GetBuiltSandwich) " ") (Utilities|String|JoinStringArray (Variables|Default|GetOrderedSandwich) " "))
    (Class|BPSandwichClientInterface|CorrectOrder(Message) _output)
    (else
      (Class|BPSandwichClientInterface|IncorrectOrder(Message) _output))))

(event Custom|CorrectSandwich
  (Class|BPSandwichClientInterface|CorrectOrder(Message) (Utilities|Array|Get(acopy) (Variables|Default|GetClientQueue))))

(event Custom|IncorrectSandwich
  (Development|PrintString "Incorrect!"))

(event EventPlayerInteracted
  (params (PlayerCharacter :type BP%20Character%20Object%20Reference))
  ;[1 1 1] Player Interaction
  (CallFunction|AddtoSandwich PlayerCharacter)
  (Default|EmptyHand PlayerCharacter))

(event EventSubmitSandwich
  ;[1 1 1] Gets called when button click
  (if (not (Utilities|Array|IsEmpty (Variables|Default|GetClientQueue)))
    (Variables|Default|SetOrderedSandwichLength (Utilities|Array|Length (Variables|Default|GetOrderedSandwich)))
    (Variables|Default|SetBadOrder? false)
    (Variables|Default|SetOrderedSandwich (Variables|/Game/_Main/Clients/Blueprints/BP_Client.BP_Client_C|GetClientOrder (Utilities|Array|Get(acopy) (Variables|Default|GetClientQueue))))
    (CallFunction|CompareSandwiches)))

(event EventAddClienttoQueue
  (params (Client :type BP%20Client%20Object%20Reference))
  ;[1 1 1] Add Client to Queue
  (Utilities|Array|Add (Variables|Default|GetClientQueue) Client))

(fn ConstructionScript
  (Variables|Default|SetNextMeshPosition (Math|Transform|MakeTransform (Math|Vector|MakeVector 0.0 0.0 (.Z (Class|KismetMathLibrary|BreakVector3f (.Max (Utilities|Struct|BreakBox (StaticMesh|GetBoundingBox (Variables|/Script/Engine.StaticMeshComponent|GetStaticMesh (Variables|Default|Get%20Plate)))))))))))