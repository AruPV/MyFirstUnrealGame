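; Game mode that starts the level timer, spawns clients and tracks the score.
; On BeginPlay it activates the first BP_Timer and spawns one BP_Client at a random BP_Spawn_Point.
; The random index uses Length - 1 as an exclusive bound, so the last spawn point found is never chosen.
; PushScoreChange adds the change to Score and forwards it to the WB_UI widget.
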(event Custom|SpawnClient
  ;[1 1 1] Spawn Client
  (bind _outactors (Actor|GetAllActorsOfClass "/Game/_Main/Clients/Blueprints/BP_Spawn_Point.BP_Spawn_Point_C"))
  (if (> (Utilities|Array|Length _outactors) 0)
    (Game|SpawnActorfromClass "/Game/_Main/Clients/Blueprints/BP_Client.BP_Client_C" (Transformation|GetActorTransform (Utilities|Array|Get(acopy) _outactors (Math|Random|RandomInteger (- (Utilities|Array|Length _outactors) 1)))) "Undefined" 0 0)))

(event EventBeginPlay
  (bind _outactors (Actor|GetAllActorsOfClass "/Game/_Main/GameTimer/BP_Timer.BP_Timer_C"))
  (Class|BPTimerActivator|ActivateTimer(Message) (Utilities|Array|Get(acopy) _outactors) 40)
  (CallFunction|SpawnClient))

(event EventPushScoreChange
  (params (ScoreChange :type Float%20%28double-precision%29))
  (Variables|Default|SetScore (+ ScoreChange (Variables|Default|GetScore)))
  (bind _foundwidgets (Widget|GetAllWidgetsOfClass "/Game/_Main/UI/WB_UI.WB_UI_C" true))
  (Default|PushScoreChange (Utilities|Array|Get(acopy) _foundwidgets) ScoreChange))

(fn ConstructionScript)