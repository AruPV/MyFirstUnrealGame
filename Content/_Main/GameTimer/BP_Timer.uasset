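; BP_Timer is a countdown timer that shows remaining time on the WB_UI widget found at BeginPlay.
; ActivateTimer sets the duration, then Tick uses a one-second Delay as a gate to decrement it until zero.
; Each step sends zero-padded MM:SS text and an urgency value, derived from remaining over total time scaled by ten, to the widget.
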(event Custom|UpdateToUI
  ;[1 1 1] UpdateUI
  (bind _urgency (CallFunction|GetUrgency))
  (bind _texttime (CallFunction|GetTimeText))
  (Class|BPTimerUIInterface|UpdateUITimer(Message) (Variables|Default|GetUI) _texttime _urgency))

(event EventTick
  (params (DeltaSeconds :type Float%20%28single-precision%29))
  ;[1 1 1] Calculate Time Remaining
  (if (Variables|Default|GetIsActivated?)
    (Utilities|FlowControl|Delay 1.0)
    (Variables|Default|SetSecondsRemaining (- (Variables|Default|GetSecondsRemaining) 1))
    (CallFunction|UpdatetoUI)
    (if (<= (Variables|Default|GetSecondsRemaining) 0)
      (Variables|Default|SetIsActivated? false))))

(event EventActivateTimer
  (params (Seconds :type Integer))
  ;[1 1 1] Activate Timer
  (bind _output_get (Variables|Default|SetSecondsTotal Seconds))
  (Variables|Default|SetSecondsRemaining _output_get)
  (Variables|Default|SetIsActivated? true))

(event EventBeginPlay
  (bind _foundwidgets (Widget|GetAllWidgetsOfClass "/Game/_Main/UI/WB_UI.WB_UI_C" true))
  (Variables|Default|SetUI (Utilities|Array|Get(acopy) _foundwidgets)))

(fn ConstructionScript)

(fn FormatTimeString
  (params (Number :type Integer))
  (bind _returnvalue (Utilities|String|ToString(Integer) Number))
  (if (> (Utilities|String|Len _returnvalue) 1)
    (return _returnvalue)
    (else
      (return (Utilities|String|Append "0" _returnvalue)))))

(fn GetTimeText
  (bind _secondsremaining (Variables|Default|GetSecondsRemaining))
  (bind _time (CallFunction|FormatTimeString (/ _secondsremaining 60)))
  (bind _time_2 (CallFunction|FormatTimeString (Math|Integer|%(Integer) _secondsremaining 60)))
  (return (Utilities|Text|ToText(String) (Utilities|String|Append _time ":" _time_2))))

(fn GetUrgency
  (return (* (/ (Variables|Default|GetSecondsRemaining) (Variables|Default|GetSecondsTotal)) 1e+01)))